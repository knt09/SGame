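; Soldier tile actor that animates its falling, attacking and getting hit through tweens.
; Falling is a speed-based, ease-out move between stored locations.
; Attacking offsets the tile along Y, swaps to the attack sprite, then chains ScaleUp, Shaking and ScaleBack through completion callbacks named by string, ending in ResetTile, which is not defined here.
; Hits play a short vertical ping-pong bump, then restore the saved location.
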(event `self.StartFalling`
  (`iTween.ActorMoveFromToFull` 0.0 "Falling" self (`self.FallingStartLocation`) (`self.FallingEndLocation`) true "none" "world" false 0.0 "first" "speed" (`self.FallingSpeed`) "easeOutCubic" null 1.0 "once" 0 "noOrientationChange" null 5.0 "none" null "" null "" null "" self))

(event `self.StartAttackAnimation`
  (`self.K2_AddActorWorldOffset` (0.0 1000.0 0.0))
  (`PaperSpriteComponent.SetSprite` (`self.RenderComponent`) (`self.Sprite_Attacking`))
  (`self.ScaleUp`))

(event `self.StartPlayHitAnimation`
  (bind _output_get (set `self.OriginalActorLocation` (`self.K2_GetActorLocation` self)))
  (`iTween.ActorMoveFromToFull` 0.0 "No Name" self _output_get (+ (`self.OriginalActorLocation`) (0.0 0.0 8.0)) true "none" "world" false 0.0 "first" "seconds" 0.05 "linear" null 1.0 "pingPong" 4 "noOrientationChange" null 5.0 "none" null "" null "" null "" self "ResetActorLocation"))

(fn `ResetActorLocation`
  (`self.K2_SetActorLocation` (`self.OriginalActorLocation`)))

(fn `ScaleBack`
  (`self.K2_SetActorRotation` (struct))
  (`iTween.ActorScaleFromToFull` 0.0 "Attacking" self (`KismetMathLibrary.Conv_DoubleToVector` (`self.AttackingScaleRatio`)) (1.0 1.0 1.0) true "none" false 0.0 "first" "seconds" (`self.AttackingScaleTimeWindow`) "linear" null 1.0 "once" 0 null "" null "" null "" self "ResetTile")
  (return))

(fn `ScaleUp`
  (`iTween.ActorScaleFromToFull` 0.0 "No Name" self (1.0 1.0 1.0) (`KismetMathLibrary.Conv_DoubleToVector` (`self.AttackingScaleRatio`)) true "none" false 0.0 "first" "seconds" (`self.AttackingScaleTimeWindow`) "linear" null 1.0 "once" 0 null "" null "" null "" self "Shaking")
  (return))

(fn `Shaking`
  (bind _attackingshakedegree (`self.AttackingShakeDegree`))
  (bind _result (`/Engine/EditorBlueprintResources/StandardMacros.NegateFloat` _attackingshakedegree)
    (:`  `
      (`iTween.ActorRotateFromToFull` 0.0 "No Name" self (`KismetMathLibrary.MakeRotator` 0.0 _attackingshakedegree) (`KismetMathLibrary.MakeRotator` 0.0 _result) true "pitchOnly" "world" false (`self.AttackingScaleTimeWindow`) "first" "seconds" 0.1 "linear" null 1.0 "pingPong" (`self.AttackingShakeFreq`) null "" null "" null "" self "ScaleBack")
      (return))))

(fn `UserConstructionScript`)