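; LinkLine_BP is a link line Blueprint that animates a ribbon between grid points and replays links.
; A delayed while-loop macro, built on RetriggerableDelay, steps both events through their points.
; The test event eases a ribbon emitter between successive static grid addresses, converted to locations by the game mode's current grid.
; The replay event calls a single-link animation for each increasing link length, printing debug text, then signals the end.
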(event `self.TestLinkLineRibbonAnimationUsingStaticPoints`
  (bind _staticlinepoints (`self.StaticLinePoints`))
  (bind _test_currentstaticpointindex (`self.Test_CurrentStaticPointIndex`))
  (`self.SetActorScale3D` (`self.LinkLineRibbonEmitter`) (1.0 1.0 1.0))
  (`self.WhileLoopWithDealy` (< (`self.Test_CurrentStaticPointIndex`) (- (`KismetArrayLibrary.Array_Length` (`self.StaticLinePoints`)) 1)) (`self.Test_SingleRibbonTime`)
    (:`Loop Body`
      (bind _assggame_mode (cast `SGGameMode` (`GameplayStatics.GetGameMode`)))
      (bind _currentgrid (`SGGameMode.CurrentGrid` _assggame_mode))
      (bind _returnvalue (`SGGrid.GetLocationFromGridAddress` _currentgrid (`KismetArrayLibrary.Array_Get` _staticlinepoints _test_currentstaticpointindex) false))
      (bind _output_get (set `self.Test_RibbonAnimationStartPos` _returnvalue))
      (bind _returnvalue_2 (`SGGrid.GetLocationFromGridAddress` _currentgrid (`KismetArrayLibrary.Array_Get` _staticlinepoints (+ _test_currentstaticpointindex 1)) true))
      (bind _output_get_2 (set `self.Test_RibbonAnimationEndPos` _returnvalue_2))
      (`iTween.ActorMoveFromToFull` 0.0 "No Name" (`self.LinkLineRibbonEmitter`) _output_get _output_get_2 true "none" "world" false 0.0 "first" "seconds" (`self.Test_SingleRibbonTime`) "easeOutCubic")
      (`/Engine/EditorBlueprintResources/StandardMacros.IncrementInt` (`self.Test_CurrentStaticPointIndex`)))))

(event `self.BeginReplayLinkAnimation`
  (bind _currentreplaylength (`self.CurrentReplayLength`))
  (set `self.CurrentReplayLength` 1)
  (`self.WhileLoopWithDealy` (< _currentreplaylength (`KismetArrayLibrary.Array_Length` (`self.LinkLinePoints`))) 0.2
    (:`Loop Body`
      (`KismetSystemLibrary.PrintText` (`KismetTextLibrary.Conv_StringToText` (`KismetStringLibrary.Concat_StrStr` "Replay Link " (`KismetStringLibrary.Conv_IntToString` _currentreplaylength))))
      (`self.ReplaySingleLinkLineAniamtion` _currentreplaylength)
      (`/Engine/EditorBlueprintResources/StandardMacros.IncrementInt` (`self.CurrentReplayLength`)))
    (:`Completed`
      (`self.EndReplayLinkAnimation`))))

(fn `UserConstructionScript`)